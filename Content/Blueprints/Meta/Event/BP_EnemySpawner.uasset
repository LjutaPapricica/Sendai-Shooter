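; BP_EnemySpawner is a level event actor that spawns a group of BP_Enemy AI pawns when triggered.
; On trigger enter, it spawns MaxEnemies pawns at random points inside the SpawnVolume box, with collision failure disabled, then signals that its logic has finished.
; The construction script sizes the spawn volume from the Extent variable.
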(event EventBeginPlay)

(event EventOnTriggerEnter
  (bind _spawnvolume (Variables|Default|GetSpawnVolume))
  (for _index (range 0 (- (Variables|Default|GetMaxEnemies) 1))
    (AI|SpawnAIFromClass "/Game/Blueprints/Pawn/AI/Zombie/BP_Enemy.BP_Enemy_C" 0 (Math|Random|RandomPointinBoundingBox (Transformation|GetWorldLocation _spawnvolume) (Components|Box|GetScaledBoxExtent _spawnvolume)) "0, 0, 0" true))
  (Default|CallOnLogicFinished))

(fn ConstructionScript
  (Components|Box|SetBoxExtent (Variables|Default|GetSpawnVolume) (Variables|Default|GetExtent) true))