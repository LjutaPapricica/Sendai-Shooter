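; Level event that fades the local player's screen to or from black when triggered.
; On trigger enter, the ToBlack flag picks the fade direction, and the first player's camera manager runs a held camera fade over FadeDuration.
; After a delay matching that duration, it calls OnLogicFinished to signal that the event is done.
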(event EventBeginPlay)

(event Collision|EventActorBeginOverlap
  (params (OtherActor :type Actor%20Object%20Reference)))

(event EventTick
  (params (DeltaSeconds :type Float%20%28single-precision%29)))

(event EventOnTriggerEnter
  (bind _returnvalue (Game|GetPlayerCameraManager 0))
  (bind _fadeduration (Variables|Default|GetFadeDuration))
  (if (Variables|Default|GetToBlack?)
    (CameraFades|StartCameraFade :self _returnvalue :ToAlpha 1.0 :Duration _fadeduration :bHoldWhenFinished true)
    (else
      (CameraFades|StartCameraFade _returnvalue 1.0 0.0 _fadeduration "(R=0.000000,G=0.000000,B=0.000000,A=1.000000)" false true)))
  (Utilities|FlowControl|Delay (Variables|Default|GetFadeDuration))
  (Default|CallOnLogicFinished))

(fn ConstructionScript
  (|CallParentFunction))