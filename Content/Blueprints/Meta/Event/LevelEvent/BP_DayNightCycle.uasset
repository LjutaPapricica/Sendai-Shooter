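; Level event that switches the scene's lighting and atmosphere in one direction when triggered, presumably between day and night.
; On trigger enter, it loops over paired directional lights, sky spheres, height fogs and post-process actors, hiding the first of each and showing the second.
; It then hides the atmospheric fog and broadcasts that its logic has finished.
; Despite the cycle name, it has no timer, blend or switch back.
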(event EventOnTriggerEnter
  (CallFunction|ChangeDayNight))

(fn ConstructionScript
  (|CallParentFunction))

(fn ChangeDayNight
  (bind _atmosphericfog (Variables|Default|GetAtmosphericFog))
  (for _index (range 0 1)
    (LocalVariables|SetIndex _index)
    (Utilities|FlowControl|Sequence
      (:then_0
        (Rendering|SetVisibility (Variables|/Script/Engine.Light|GetLightComponent (Utilities|Array|Get(acopy) (Variables|Default|GetDirectionalLights) (LocalVariables|GetIndex))) (!= (LocalVariables|GetIndex) 0) false)
        (Rendering|SetActorHiddenInGame (Utilities|Array|Get(acopy) (Variables|Default|GetDirectionalLights) (LocalVariables|GetIndex)) (== (LocalVariables|GetIndex) 0)))
      (:then_1
        (Rendering|SetVisibility (Variables|/Engine/EngineSky/BP_Sky_Sphere.BP_Sky_Sphere_C|GetBase (Utilities|Array|Get(acopy) (Variables|Default|GetSkySpheres) (LocalVariables|GetIndex))) (!= (LocalVariables|GetIndex) 0) false)
        (Rendering|SetActorHiddenInGame (Utilities|Array|Get(acopy) (Variables|Default|GetSkySpheres) (LocalVariables|GetIndex)) (== (LocalVariables|GetIndex) 0)))
      (:then_2
        (Rendering|SetVisibility (Variables|/Script/Engine.ExponentialHeightFog|GetComponent (Utilities|Array|Get(acopy) (Variables|Default|GetHeightFogs) (LocalVariables|GetIndex))) (!= (LocalVariables|GetIndex) 0) false)
        (Rendering|SetActorHiddenInGame (Utilities|Array|Get(acopy) (Variables|Default|GetHeightFogs) (LocalVariables|GetIndex)) (== (LocalVariables|GetIndex) 0)))
      (:then_3
        (Rendering|SetActorHiddenInGame (Utilities|Array|Get(acopy) (Variables|Default|GetPostProcessActors) (LocalVariables|GetIndex)) (== (LocalVariables|GetIndex) 0)))))
  (Utilities|FlowControl|Sequence
    (:then_0
      (Rendering|SetVisibility (Variables|/Script/Engine.AtmosphericFog|GetAtmosphericFogComponent _atmosphericfog) false false)
      (Rendering|SetActorHiddenInGame _atmosphericfog true))
    (:then_1
      (Default|CallOnLogicFinished))))