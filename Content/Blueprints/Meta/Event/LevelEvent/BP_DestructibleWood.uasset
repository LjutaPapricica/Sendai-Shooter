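; BP_DestructibleWood is a level event that shatters wooden destructible pieces and drops the player into ragdoll.
; On trigger enter, it enables physics on four destructible components and applies heavy damage to each with an impulse along its negative up vector.
; When the component named Destructible fractures, it ragdolls the ALS shooter player character and signals that the event logic has finished.
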(event OnComponentFracture(Destructible)
  (params (HitPoint :type Vector%20%28by%20ref%29 :default "0, 0, 0") (HitDirection :type Vector%20%28by%20ref%29 :default "0, 0, 0"))
  (bind _asals_player_shooter_character_bp (Utilities|Casting|CastToALS_Player_ShooterCharacterBP (Game|Player|GetPlayerPawn 0)))
  (Default|EventRagdoll _asals_player_shooter_character_bp true)
  (Default|CallOnLogicFinished))

(event EventBeginPlay
  (Variables|Default|SetMeshs (Utilities|Array|MakeArray (Variables|Default|GetDestructible1) (Variables|Default|GetDestructible2) (Variables|Default|GetDestructible3) (Variables|Default|GetDestructible))))

(event EventOnTriggerEnter
  (for _array_element (Variables|Default|GetMeshs)
    (Physics|SetSimulatePhysics _array_element true)
    (Class|DestructibleComponent|ApplyDamage _array_element 1e+04 (Transformation|GetWorldLocation _array_element) (* (Math|Vector|GetUpVector (Transformation|GetWorldRotation _array_element)) -1.0) 1e+03)))

(fn ConstructionScript
  (|CallParentFunction))