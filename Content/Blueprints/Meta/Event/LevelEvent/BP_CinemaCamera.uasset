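; BP_CinemaCamera is a level event camera that temporarily takes over the first player's view when triggered.
; It blends the view to itself with a cubic blend over BlendTime, then signals that its logic has finished and holds for WaitTime.
; ReturnToPlayerCamera then blends back to the player pawn over a fixed duration.
; The c_ReturnInput event can call that return directly, without waiting for the delays.
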(event Custom|c_ReturnInput
  (CallFunction|ReturntoPlayerCamera))

(event EventOnTriggerEnter
  (bind _blendtime (Variables|Default|GetBlendTime))
  (Game|Player|SetViewTargetwithBlend (Game|GetPlayerController 0) self _blendtime "VTBlend_Cubic" 0.0 false)
  (Utilities|FlowControl|Delay _blendtime)
  (Default|CallOnLogicFinished)
  (Utilities|FlowControl|Delay (Variables|Default|GetWaitTime))
  (CallFunction|ReturntoPlayerCamera))

(fn ConstructionScript
  (|CallParentFunction))

(fn ReturntoPlayerCamera
  (Game|Player|SetViewTargetwithBlend (Game|GetPlayerController 0) (Game|Player|GetPlayerPawn 0) 1.0 "VTBlend_Linear" 0.0 false))