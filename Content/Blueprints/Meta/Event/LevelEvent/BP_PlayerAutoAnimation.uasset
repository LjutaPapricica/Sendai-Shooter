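; BP_PlayerAutoAnimation is a level event that automatically walks the player pawn to a destination once triggered.
; Each tick it feeds half-scale movement input toward Destination, an offset from the actor's location, using a look-at rotation's forward vector.
; When the pawn comes within tolerance of that point, a DoOnce stops the movement and calls OnLogicFinished.
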(event EventOnTriggerEnter
  (Variables|Default|SetCanMove true))

(event EventTick
  (params (DeltaSeconds :type Float%20%28single-precision%29))
  (bind _returnvalue (Game|Player|GetPlayerPawn 0))
  (if (Variables|Default|GetCanMove)
    (if (Math|Vector|Equal(Vector) (+ (Variables|Default|GetDestination) (Transformation|GetActorLocation)) (Transformation|GetActorLocation (Game|Player|GetPlayerPawn 0)) 1e+02)
      (Utilities|FlowControl|DoOnce false
        (:Completed
          (Variables|Default|SetCanMove false)
          (Default|CallOnLogicFinished)))
      (else
        (Pawn|Input|AddMovementInput _returnvalue (Math|Vector|GetForwardVector (Math|Rotator|FindLookatRotation (Transformation|GetActorLocation _returnvalue) (+ (Variables|Default|GetDestination) (Transformation|GetActorLocation)))) 0.5 false)))))

(fn ConstructionScript
  (|CallParentFunction))