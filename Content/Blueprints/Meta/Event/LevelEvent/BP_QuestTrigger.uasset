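; BP_QuestTrigger is a level event trigger that toggles the quest-item state of a usable item.
; On trigger enter and end, it finds the first actor of the QuestActor class, casts it to BP_Base_UsableItem and sets or clears IsQuestItem.
; Both paths then call CallOnLogicFinished and DoRemoteEvent, which are skipped if the cast fails.
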(event EventBeginPlay)

(event Collision|EventActorBeginOverlap
  (params (OtherActor :type Actor%20Object%20Reference)))

(event EventTick
  (params (DeltaSeconds :type Float%20%28single-precision%29)))

(event EventOnTriggerEnter
  (bind _outactors (Actor|GetAllActorsOfClass (Variables|Default|GetQuestActor)))
  (bind _asbp_base_usable_item (Utilities|Casting|CastToBP_Base_UsableItem (Utilities|Array|Get(acopy) _outactors)))
  (Variables|/Game/Blueprints/Actor/Item/Usable/BP_Base_UsableItem.BP_Base_UsableItem_C|SetisQuestItem _asbp_base_usable_item true)
  (Default|CallOnLogicFinished)
  (CallFunction|DoRemoteEvent))

(event EventOnTriggerEnd
  (bind _outactors (Actor|GetAllActorsOfClass (Variables|Default|GetQuestActor)))
  (bind _asbp_base_usable_item (Utilities|Casting|CastToBP_Base_UsableItem (Utilities|Array|Get(acopy) _outactors)))
  (Variables|/Game/Blueprints/Actor/Item/Usable/BP_Base_UsableItem.BP_Base_UsableItem_C|SetisQuestItem _asbp_base_usable_item false)
  (Default|CallOnLogicFinished)
  (CallFunction|DoRemoteEvent))

(fn ConstructionScript
  (|CallParentFunction))