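; BP_EventInstigator is a box trigger that runs a chain of event actors when the player pawn overlaps it.
; A CanThrough-gated DoOnce starts the active entry in EventActors, and end overlap notifies that entry.
; Each actor's OnLogicFinished advances the index and triggers the next, guarded by an array bounds check.
; A remote event resets and re-fires the DoOnce, and the construction script sizes the box from Extent.
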(event OnComponentBeginOverlap(EventTrigger)
  (params (OverlappedComponent :type Primitive%20Component%20Object%20Reference) (OtherActor :type Actor%20Object%20Reference) (OtherComp :type Primitive%20Component%20Object%20Reference) (OtherBodyIndex :type Integer) (bFromSweep :type Boolean) (SweepResult :type Hit%20Result%20Structure%20%28by%20ref%29))
  (if (and (== OtherActor (Game|Player|GetPlayerPawn 0)) (Variables|Default|GetCanThrough))
    (Utilities|FlowControl|DoOnce false
      (:Completed
        (Default|OnTriggerEnter (Utilities|Array|Get(acopy) (Variables|Default|GetEventActors) (Variables|Default|GetActiveIndex)))))))

(event OnComponentEndOverlap(EventTrigger)
  (params (OverlappedComponent :type Primitive%20Component%20Object%20Reference) (OtherActor :type Actor%20Object%20Reference) (OtherComp :type Primitive%20Component%20Object%20Reference) (OtherBodyIndex :type Integer))
  (Default|OnTriggerEnd (Utilities|Array|Get(acopy) (Variables|Default|GetEventActors) (Variables|Default|GetActiveIndex))))

(event Custom|c_RemoteEvent
  (Utilities|FlowControl|Sequence
    (:then_0
      (goto _label Reset))
    (:then_1
      (Utilities|FlowControl|DoOnce false :!label _label
        (:Completed
          (Default|OnTriggerEnter (Utilities|Array|Get(acopy) (Variables|Default|GetEventActors) (Variables|Default|GetActiveIndex))))))))

(event Custom|OnLogicFinished_Event_0
  (if (|CheckArrayExist)
    (Math|Integer|IncrementInt (Variables|Default|GetActiveIndex)
      (:%20%20
        (Default|OnTriggerEnter (Utilities|Array|Get(acopy) (Variables|Default|GetEventActors) (Variables|Default|GetActiveIndex)))))))

(event EventBeginPlay
  (for _array_element (Variables|Default|GetEventActors)
    (EventDispatchers|AssignOnLogicFinished _array_element (delegate Custom|OnLogicFinished_Event_0))))

(fn ConstructionScript
  (Components|Box|SetBoxExtent (Variables|Default|GetEventTrigger) (Variables|Default|GetExtent) false))