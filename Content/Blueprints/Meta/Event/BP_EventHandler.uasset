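; BP_EventHandler tracks an objective to pick up a set number of important items, then unlocks event instigators.
; On BeginPlay it shows the objective widget and registers itself on the player's ALS shooter character.
; HasPickedupImpItem decrements the remaining count, which a looping timer polls every few seconds.
; At zero it removes the widget and sets CanThrough on each instigator; the timer is never cleared.
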(event EventBeginPlay
  (Utilities|FlowControl|Sequence
    (:then_0
      (bind _returnvalue (UserInterface|CreateWidget "/Game/Blueprints/UI/BPUI_Objective.BPUI_Objective_C"))
      (bind _output_get (Variables|Default|SetUI_Objective _returnvalue))
      (UserInterface|Viewport|AddtoViewport _output_get 0))
    (:then_1
      (bind _asals_player_shooter_character_bp (Utilities|Casting|CastToALS_Player_ShooterCharacterBP (Game|Player|GetPlayerPawn 0)))
      (Variables|/Game/AdvancedLocomotionV2/Blueprints/ALS_Shooter/ALS_Player_ShooterCharacterBP.ALS_Player_ShooterCharacterBP_C|SetEventHandler _asals_player_shooter_character_bp self))
    (:then_2
      (Utilities|Time|SetTimerbyFunctionName 0 "CheckAllItemsHasPickedUp" 3.0 true))))

(fn ConstructionScript)

(fn HasPickedupImpItem
  (Math|Integer|DecrementInt (Variables|Default|GetNumOfNeedItems)))

(fn CheckAllItemsHasPickedUp
  (if (== (Variables|Default|GetNumOfNeedItems) 0)
    (Utilities|FlowControl|Sequence
      (:then_0
        (Widget|RemovefromParent (Variables|Default|GetUI_Objective)))
      (:then_1
        (for _array_element (Variables|Default|GetEventInstigators)
          (Variables|/Game/Blueprints/Meta/Event/BP_EventInstigator.BP_EventInstigator_C|SetCanThrough _array_element true))))))