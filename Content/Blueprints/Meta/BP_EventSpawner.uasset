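; BP_EventSpawner is a trigger-based enemy spawner that populates an area once the player enters it.
; When the player pawn first overlaps the Trigger box, a DoOnce gate fires a loop that spawns MaxEnemies BP_Enemy AI pawns.
; Each spawns at a random point inside the EnemySpawnVolume box, ignoring collision failures.
; The construction script sizes the Trigger from the BoxExtent variable.
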(event OnComponentBeginOverlap(Trigger)
  (params (OverlappedComponent :type Primitive%20Component%20Object%20Reference) (OtherActor :type Actor%20Object%20Reference) (OtherComp :type Primitive%20Component%20Object%20Reference) (OtherBodyIndex :type Integer) (bFromSweep :type Boolean) (SweepResult :type Hit%20Result%20Structure%20%28by%20ref%29))
  (bind _enemyspawnvolume (Variables|Default|GetEnemySpawnVolume))
  (if (== OtherActor (Game|Player|GetPlayerPawn 0))
    (Utilities|FlowControl|DoOnce false
      (:Completed
        (for _index (range 0 (- (Variables|Default|GetMaxEnemies) 1))
          (AI|SpawnAIFromClass "/Game/Blueprints/Pawn/AI/Zombie/BP_Enemy.BP_Enemy_C" 0 (Math|Random|RandomPointinBoundingBox (Transformation|GetWorldLocation _enemyspawnvolume) (Components|Box|GetScaledBoxExtent _enemyspawnvolume)) "0, 0, 0" true))))))

(event EventBeginPlay)

(event Collision|EventActorBeginOverlap
  (params (OtherActor :type Actor%20Object%20Reference)))

(event EventTick
  (params (DeltaSeconds :type Float%20%28single-precision%29)))

(fn ConstructionScript
  (Components|Box|SetBoxExtent (Variables|Default|GetTrigger) (Variables|Default|GetBoxExtent) true))