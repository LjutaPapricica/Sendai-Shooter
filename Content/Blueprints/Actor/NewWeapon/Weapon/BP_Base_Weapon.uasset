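; Base weapon actor for assault rifle and shotgun types, handling pickup, socket-based equipping, firing and reloading for the ALS shooter player.
; Firing runs multi line traces with growing random spread, reducing damage per penetration until a blocking hit and spawning surface-based impacts, bullet holes or body damage.
; Rifles support full or semi auto and magazine reloads; shotguns fire pellet loops and replay their montage to load shell by shell.
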(event OnComponentBeginOverlap(InteractTrigger)
  (params (OverlappedComponent :type Primitive%20Component%20Object%20Reference) (OtherActor :type Actor%20Object%20Reference) (OtherComp :type Primitive%20Component%20Object%20Reference) (OtherBodyIndex :type Integer) (bFromSweep :type Boolean) (SweepResult :type Hit%20Result%20Structure%20%28by%20ref%29))
  ;[1 1 1] Box Overlap
  (if (== OtherActor (Game|Player|GetPlayerPawn 0))
    (Class|BPIInteract|SetCanPickUp(Message) OtherActor true)))

(event OnComponentEndOverlap(InteractTrigger)
  (params (OverlappedComponent :type Primitive%20Component%20Object%20Reference) (OtherActor :type Actor%20Object%20Reference) (OtherComp :type Primitive%20Component%20Object%20Reference) (OtherBodyIndex :type Integer))
  ;[1 1 1] Box Overlap
  (if (== OtherActor (Game|Player|GetPlayerPawn 0))
    (Class|BPIInteract|SetCanPickUp(Message) OtherActor false)))

(event EventWeaponHasInteracted
  (params (ParentComp :type Scene%20Component%20Object%20Reference) (AttachSocketName :type Name :default "None"))
  ;[1 1 1] When weapon interact
  (CallFunction|PickUp ParentComp AttachSocketName))

(event EventTick
  (params (DeltaSeconds :type Float%20%28single-precision%29))
  ;[1 1 1] debug
)

(event EventBeginPlay
  (bind _returnvalue (Game|Player|GetPlayerPawn 0))
  (bind _returnvalue_2 (Actor|GetComponentbyClass _returnvalue "/Script/Engine.SkeletalMeshComponent"))
  ;[1 1 1] BeginPlay
  (Utilities|FlowControl|Sequence
    (:then_0
      (bind _asals_player_shooter_character_bp (Utilities|Casting|CastToALS_Player_ShooterCharacterBP (Game|Player|GetPlayerPawn 0)))
      (Variables|Reference|SetPlayerRefe _asals_player_shooter_character_bp))
    (:then_1
      (Variables|Reference|SetPlayerAnimInst (Components|SkeletalMesh|GetAnimInstance _returnvalue_2)))
    (:then_2
      (Variables|Default|SetSkeletalMesh _returnvalue_2))
    (:then_3
      (Variables|Integer|SetMaxAmmo (* (Variables|Integer|GetAmmo) 2)))))

(fn ConstructionScript)

(fn PickUp
  (params (ToAttachComp :type Scene%20Component%20Object%20Reference) (SocketName :type Name))
  (Collision|SetCollisionEnabled (Variables|Default|GetWeaponMesh) "NoCollision")
  (Transformation|AttachComponentToComponent (Variables|Default|GetWeaponMesh) ToAttachComp SocketName "SnapToTarget" "SnapToTarget" "SnapToTarget" true))

(fn Equip
  (params (ToAttachComp :type Scene%20Component%20Object%20Reference))
  (Transformation|DetachFromComponent (Variables|Default|GetWeaponMesh) "KeepWorld" "KeepWorld" "KeepWorld" true)
  (Transformation|AttachComponentToComponent (Variables|Default|GetWeaponMesh) ToAttachComp (Variables|Name|GetGrabSocketName) "SnapToTarget" "SnapToTarget" "SnapToTarget" true)
  (Variables|Bool|SetEquiping true))

(fn UnEquip
  (params (ToAttachComp :type Scene%20Component%20Object%20Reference) (SocketName :type Name))
  (Transformation|DetachFromComponent (Variables|Default|GetWeaponMesh) "KeepWorld" "KeepWorld" "KeepWorld" true)
  (Transformation|AttachComponentToComponent (Variables|Default|GetWeaponMesh) ToAttachComp SocketName "SnapToTarget" "SnapToTarget" "SnapToTarget" true)
  (Variables|Bool|SetEquiping false))

(fn FireTrace
  (bind (_start _end) (|GetTraceStart/End))
  (bind _maxbulletspread (Variables|Vector|GetMaxBulletSpread))
  (bind _playerrefe (Variables|Reference|GetPlayerRefe))
  (bind _spreadcurrent (Variables|/Game/AdvancedLocomotionV2/Blueprints/ALS_Shooter/ALS_Player_ShooterCharacterBP.ALS_Player_ShooterCharacterBP_C|GetSpreadCurrent _playerrefe))
  (Default|IncreaseSpread (Variables|Reference|GetPlayerRefe) (Variables|Float|GetBulletSpradAmount))
  (bind (_outhits _returnvalue) (Collision|MultiLineTraceByChannel _start (+ _end (Math|Vector|MakeVector 0.0 (* (Math|Random|RandomFloatinRange (* (.x _maxbulletspread) -1.0) (.x _maxbulletspread)) _spreadcurrent) (* (Math|Random|RandomFloatinRange (* (.y _maxbulletspread) -1.0) (.y _maxbulletspread)) _spreadcurrent))) "TraceTypeQuery1" false (Utilities|Array|MakeArray (Game|Player|GetPlayerPawn 0)) "None"))
  (if _returnvalue
    (|SetHitResult _outhits :!label _label
      (:then_3
        (|SpawnEmitter)
        (|AddDamage)
        (if (Variables|Bool|GetHasBlocked)
          (|SetDamageToInitialDamage)
          (goto _label Break)
          (else
            (|DamageDecrease)))))))

(fn GrabMagazine
  (Transformation|AttachComponentToComponent (Variables|Default|GetMagazine) (Variables|Default|GetSkeletalMesh) "MagazineGrabSocket" "SnapToTarget" "SnapToTarget" "SnapToTarget" true))

(fn ReleaseMagazine
  (bind _returnvalue (Transformation|AttachComponentToComponent (Variables|Default|GetMagazine) (Variables|Default|GetWeaponMesh) "MagazineSocket" "KeepRelative" "KeepRelative" "KeepWorld" true))
  (if _returnvalue
    (CallFunction|CRelaodAmmo)))

(fn PickUpAmmo
  (Variables|Integer|SetMaxAmmo (+ (Variables|Integer|GetMaxAmmo) (Utilities|Select :Index (Variables|Enum|GetEWeaponType) :NewEnumerator0 30 :NewEnumerator1 7))))

(event Custom|ResetSGReload
  (Utilities|FlowControl|DoN (- (Variables|Integer|GetInitialAmmo) (Variables|Integer|GetAmmo))) ; enters at Reset
)

(event Custom|c_RelaodAmmo
  (switch Utilities|FlowControl|Switch|Switchone_WeaponType (Variables|Enum|GetEWeaponType)
    (:NewEnumerator0
      (|ARReload))
    (:NewEnumerator1
      (|SGReload))))

(event EventReload
  (if (|CanReloadCondition)
    (switch Utilities|FlowControl|Switch|Switchone_WeaponType (Variables|Enum|GetEWeaponType) :!label _label
      (:NewEnumerator0
        (Animation|Montage|MontagePlay (Variables|Reference|GetPlayerAnimInst) (Variables|Montage|GetReloadMontage) 1.0 "MontageLength" 0.0))
      (:NewEnumerator1
        (Animation|Montage|PlayMontage (Variables|Default|GetSkeletalMesh) (Variables|Montage|GetReloadMontage) 2.0
          (:OnCompleted
            (if (> (Variables|Integer|GetMaxAmmo) 0)
              (Utilities|FlowControl|DoN (- (Variables|Integer|GetInitialAmmo) (Variables|Integer|GetAmmo)) :!label _label_2
                (:Exit
                  (goto _label)))))
          (:OnInterrupted
            (goto _label_2 Reset)))))))

(event Custom|c_Fire
  (switch Utilities|FlowControl|Switch|Switchone_WeaponType (Variables|Enum|GetEWeaponType)
    (:NewEnumerator0
      _)
    (:NewEnumerator1
      (Utilities|FlowControl|DoOnce false
        (:Completed
          _))))
  (if (|CanShootCondition)
    (Utilities|FlowControl|Sequence
      (:then_0
        (Utilities|FlowControl|DoOnce))
      (:then_1
        (switch Utilities|FlowControl|Switch|Switchone_WeaponType (Variables|Enum|GetEWeaponType)
          (:NewEnumerator0
            (switch Utilities|FlowControl|Switch|Switchone_FireLogic (Variables|Enum|GetEFireLogic)
              (:NewEnumerator0
                (CallFunction|FireTrace :!label _label)
                (Utilities|FlowControl|Delay (/ 1.0 (Variables|Float|GetFireRate)))
                (if (Variables|Bool|GetShooting)
                  (CallFunction|CFire)
                  (goto _label)))
              (:NewEnumerator1
                (CallFunction|FireTrace))))
          (:NewEnumerator1
            (for _index (range 0 9)
              (CallFunction|FireTrace)
              (Utilities|FlowControl|Delay (Variables|Float|GetFireRate))
              (CallFunction|CAllowNextFire))))))
    (else
      (Variables|Bool|SetShooting false))))

(event Custom|c_AllowNextFire
  (Utilities|FlowControl|DoOnce false) ; enters at Reset
)

(event EventFireStop
  (Variables|Bool|SetShooting false)
  (if (Variables|Bool|GetShooting) :!label _label
    (CallFunction|CFire)
    (CallFunction|FireTrace)
    (Utilities|FlowControl|Delay (/ 1.0 (Variables|Float|GetFireRate)))
    (goto _label)))

(event EventFireStart
  (Variables|Bool|SetShooting true)
  (CallFunction|CFire))