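; Base weapon actor that the player can pick up, equip and unequip by attaching its mesh to sockets.
; An interact trigger toggles the player pawn's pickup message on overlap, and the interaction event calls PickUp, which disables mesh and trigger collision and snaps the mesh to the given socket.
; Equip and UnEquip detach the mesh and reattach it to the grab socket or a supplied socket, respectively.
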(event OnComponentBeginOverlap(InteractTrigger)
  (params (OverlappedComponent :type Primitive%20Component%20Object%20Reference) (OtherActor :type Actor%20Object%20Reference) (OtherComp :type Primitive%20Component%20Object%20Reference) (OtherBodyIndex :type Integer) (bFromSweep :type Boolean) (SweepResult :type Hit%20Result%20Structure%20%28by%20ref%29))
  (if (== OtherActor (Game|Player|GetPlayerPawn 0))
    (Class|BPIInteract|SetCanPickUp(Message) OtherActor true)))

(event OnComponentEndOverlap(InteractTrigger)
  (params (OverlappedComponent :type Primitive%20Component%20Object%20Reference) (OtherActor :type Actor%20Object%20Reference) (OtherComp :type Primitive%20Component%20Object%20Reference) (OtherBodyIndex :type Integer))
  (if (== OtherActor (Game|Player|GetPlayerPawn 0))
    (Class|BPIInteract|SetCanPickUp(Message) OtherActor false)))

(event EventWeaponHasInteracted
  (params (ParentComp :type Scene%20Component%20Object%20Reference) (AttachSocketName :type Name :default "None"))
  (CallFunction|PickUp ParentComp AttachSocketName))

(fn ConstructionScript)

(fn PickUp
  (params (ToAttachComp :type Scene%20Component%20Object%20Reference) (SocketName :type Name))
  (Collision|SetCollisionEnabled (Variables|Default|GetWeaponMesh) "NoCollision")
  (Transformation|AttachComponentToComponent (Variables|Default|GetWeaponMesh) ToAttachComp SocketName "SnapToTarget" "SnapToTarget" "SnapToTarget" true))

(fn Equip
  (params (ToAttachComp :type Scene%20Component%20Object%20Reference))
  (Transformation|DetachFromComponent (Variables|Default|GetWeaponMesh) "KeepWorld" "KeepWorld" "KeepWorld" true)
  (Transformation|AttachComponentToComponent (Variables|Default|GetWeaponMesh) ToAttachComp (Variables|Default|GetGrabSocketName) "SnapToTarget" "SnapToTarget" "SnapToTarget" true))

(fn UnEquip
  (params (ToAttachComp :type Scene%20Component%20Object%20Reference) (SocketName :type Name))
  (Transformation|DetachFromComponent (Variables|Default|GetWeaponMesh) "KeepWorld" "KeepWorld" "KeepWorld" true)
  (Transformation|AttachComponentToComponent (Variables|Default|GetWeaponMesh) ToAttachComp SocketName "SnapToTarget" "SnapToTarget" "KeepWorld" true))