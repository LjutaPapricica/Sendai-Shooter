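; BP_Base_CartRidge is a base weapon cartridge actor that launches itself as a physics object when spawned.
; On BeginPlay it enables physics simulation on its mesh, then applies a randomized impulse along player pawn 0's right vector plus an upward world-Z component.
; The impulse direction always follows that pawn rather than the spawning weapon, and it is mass-dependent because velocity change is off.
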(event EventBeginPlay
  (Utilities|FlowControl|Sequence
    (:then_0
      (Physics|SetSimulatePhysics (Variables|Default|GetCartRidgeMesh) true))
    (:then_1
      (Physics|AddImpulse (Variables|Default|GetCartRidgeMesh) (+ (* (Transformation|GetActorRightVector (Game|Player|GetPlayerPawn 0)) (Math|Random|RandomFloatinRange 3.0 8.0)) (Math|Vector|MakeVector 0.0 0.0 (Math|Random|RandomFloatinRange 15.0 25.0))) "None" false))))

(fn ConstructionScript)