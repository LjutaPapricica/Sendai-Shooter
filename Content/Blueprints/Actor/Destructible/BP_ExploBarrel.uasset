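; Explosive barrel that blows up once when damaged, spawning explosion effects and sound.
; The Explosion timeline is meant to grow DamageSphere, then destroy the actor after a short delay.
; Sphere overlaps apply radial falloff damage to enemies and push physics-simulating bodies outward.
; Overlaps also collapse BP_Log actors and forward damage to other BP_Dest destructibles, allowing chain reactions.
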(event OnComponentBeginOverlap(DamageSphere)
  (params (OverlappedComponent :type Primitive%20Component%20Object%20Reference) (OtherActor :type Actor%20Object%20Reference) (OtherComp :type Primitive%20Component%20Object%20Reference) (OtherBodyIndex :type Integer) (bFromSweep :type Boolean) (SweepResult :type Hit%20Result%20Structure%20%28by%20ref%29))
  (bind _asbp_enemy (Utilities|Casting|CastToBP_Enemy OtherActor)
    (:then
      (Class|GameplayStatics|ApplyRadialDamagewithFalloff _asbp_enemy 1e+02 3e+01 (Transformation|GetActorLocation) 2e+02 5e+02 0.23333333 0 0 0 0 "ECC_Visibility")
      (if (Physics|IsSimulatingPhysics (Variables|/Script/Engine.Character|GetMesh _asbp_enemy) "None")
        (Physics|AddImpulse (Variables|/Script/Engine.Character|GetMesh _asbp_enemy) (* (Math|Vector|GetForwardVector (Math|Rotator|FindLookatRotation (Transformation|GetActorLocation) (Transformation|GetActorLocation _asbp_enemy))) (Variables|Default|GetImpulse)) "None" false)))
    (:CastFailed
      (bind _asbp_log (Utilities|Casting|CastToBP_Log OtherActor)
        (:then
          (Default|CollapseLog _asbp_log))
        (:CastFailed
          (bind _asbp_dest (Utilities|Casting|CastToBP_Dest OtherActor))
          (Default|HasTakenDamage _asbp_dest))))))

(event EventHasTakenDamage
  (Utilities|FlowControl|DoOnce false
    (:Completed
      (CallFunction|SpawnFX/Sound "/Game/Sound/Explosion/Explosion_Cue.Explosion_Cue" "/Game/Effects/Particles/P_Explosion.P_Explosion" (+ (Transformation|GetWorldLocation (Variables|Default|GetBarrel)) "0, 0,100.000000") "3.000000,3.000000,3.000000")
      (Audio|Components|Audio|Play (Variables|Default|GetExplosion)))))

(fn ConstructionScript
  (|CallParentFunction))