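; BP_Log is a destructible pile of seven logs, with randomized meshes, that collapses to damage enemies.
; CollapseLog enables physics once and launches the logs forward and upward from an arrow-like direction component.
; Fast log hits damage BP_Enemy and push its mesh if ragdolled.
; Three seconds after an enemy hit, logs switch to physics-only collision and stop dealing damage; the max-velocity debug print is unused.
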(event Custom|CollapseLog
  (Utilities|FlowControl|DoOnce false
    (:Completed
      (for _array_element (Variables|Default|GetLogs)
        (Physics|SetSimulatePhysics _array_element true)
        (Physics|AddImpulse _array_element (+ (* (Math|Vector|GetForwardVector (Transformation|GetWorldRotation (Variables|Default|GetImpuseApplyForward))) 1.3e+04) "0, 0,15000.000000") "None" false)))))

(event Collision|EventHit
  (params (MyComp :type Primitive%20Component%20Object%20Reference) (Other :type Actor%20Object%20Reference) (OtherComp :type Primitive%20Component%20Object%20Reference) (bSelfMoved :type Boolean) (HitLocation :type Vector :default "0, 0, 0") (HitNormal :type Vector :default "0, 0, 0") (NormalImpulse :type Vector :default "0, 0, 0") (Hit :type Hit%20Result%20Structure%20%28by%20ref%29))
  (bind _returnvalue (Transformation|GetComponentVelocity MyComp))
  (bind (_x _y _z) (Math|Vector|BreakVector _returnvalue))
  (bind _returnvalue_2 (Math|Float|Absolute(Float) _z))
  (bind _returnvalue_3 (Math|Float|Absolute(Float) _x))
  (bind _returnvalue_4 (Math|Float|Absolute(Float) _y))
  (bind _returnvalue_5 (+ _returnvalue_3 _returnvalue_4 _returnvalue_2))
  (bind _returnvalue_6 (* _returnvalue_5 2.5e+02))
  (bind _asbp_enemy (Utilities|Casting|CastToBP_Enemy Other))
  (if (Variables|Default|GetisLogActive)
    (if (>= _returnvalue_6 5e+04)
      (Game|Damage|ApplyDamage _asbp_enemy 1e+02 0 0)
      (if (Physics|IsSimulatingPhysics (Variables|/Script/Engine.Character|GetMesh _asbp_enemy) "None")
        (Physics|AddImpulse (Variables|/Script/Engine.Character|GetMesh _asbp_enemy) (* (Math|Vector|GetForwardVector (Transformation|GetWorldRotation (Variables|Default|GetImpuseApplyForward))) (* _returnvalue_6 0.05)) "None" false)))
    (Utilities|FlowControl|Delay 3.0)
    (Utilities|FlowControl|DoOnce false
      (:Completed
        (for _array_element (Variables|Default|GetLogs)
          (Collision|SetCollisionEnabled _array_element "PhysicsOnly"))
        (Variables|Default|SetisLogActive false)))))

(event EventBeginPlay
  (Variables|Default|SetLogs (Utilities|Array|MakeArray (Variables|Default|GetLog_1) (Variables|Default|GetLog_2) (Variables|Default|GetLog_3) (Variables|Default|GetLog_4) (Variables|Default|GetLog_5) (Variables|Default|GetLog_6) (Variables|Default|GetLog_7))))

(fn ConstructionScript
  (for _array_element (Utilities|Array|MakeArray (Variables|Default|GetLog_1) (Variables|Default|GetLog_2) (Variables|Default|GetLog_3) (Variables|Default|GetLog_4) (Variables|Default|GetLog_5) (Variables|Default|GetLog_6) (Variables|Default|GetLog_7))
    (Components|StaticMesh|SetStaticMesh _array_element (Utilities|Array|Get(acopy) (Variables|Default|GetLog_Meshs) (Math|Random|RandomIntegerinRange 0 3)))))