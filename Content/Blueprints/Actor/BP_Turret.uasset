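; Automated gun turret that sweeps back and forth, then tracks and shoots characters it detects, until destroyed.
; Each tick a sphere trace feeds target detection and delayed hitscan fire, while SearchingEnemy handles yaw sweep, interpolated chase and return to initial rotation.
; A retriggerable delay serves as target memory, and taking damage targets the attacking character.
; At zero HP it becomes a physics wreck with an impulse and limited lifespan.
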(event EventBeginPlay
  (Utilities|FlowControl|Sequence
    (:then_0
      (|SetClampRotation))
    (:then_1
      (|SetInitialRotation))))

(event EventApplyDamage
  (params (Damage :type Float%20%28single-precision%29) (DamageCauser :type Actor%20Object%20Reference))
  (|DrainHP Damage DamageCauser)
  (|DeadLogic))

(event EventTick
  (params (DeltaSeconds :type Float%20%28single-precision%29))
  (Utilities|FlowControl|Sequence
    (:then_0
      (|SphereTrace))
    (:then_1
      (|SearchingEnemy))))

(fn ConstructionScript)