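; Zombie spawn point actor that spawns BP_StrongZombieAI pawns at its root location.
; BeginPlay starts a looping timer with a random interval picked once, spawning one zombie per tick until the count reaches MaxEnemies.
; c_StopSpawning clears the timer and resets the count, while c_StartSpawning is an empty event, so nothing here restarts spawning.
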(event Custom|c_SpawnZombie
  (if (!= (Variables|Default|GetNumofEnemies) (Variables|Default|GetMaxEnemies))
    (AI|SpawnAIFromClass "/Game/Blueprints/Pawn/AI/Zombie/BP_StrongZombieAI.BP_StrongZombieAI_C" 0 (Transformation|GetWorldLocation (Variables|Default|GetDefaultSceneRoot)) "0, 0, 0" false)
    (Math|Integer|IncrementInt (Variables|Default|GetNumofEnemies))))

(event Custom|c_StartSpawning)

(event Custom|c_StopSpawning
  (Utilities|Time|ClearTimerbyFunctionName 0 "c_SpawnZombie")
  (Variables|Default|SetNumofEnemies 0))

(event EventBeginPlay
  (Utilities|Time|SetTimerbyFunctionName 0 "c_SpawnZombie" (Math|Random|RandomFloatinRange 3.0 1e+01) true))

(fn ConstructionScript)