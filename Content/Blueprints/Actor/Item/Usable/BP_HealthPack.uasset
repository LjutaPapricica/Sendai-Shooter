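; BP_HealthPack is a usable item that restores health to the player.
; On use it casts player pawn 0 to ALS_Player_ShooterCharacterBP, calls PickedUpHealth with a fixed amount and plays a 2D heal sound.
; Once interacted with, it disables collision on its sphere and mesh.
; Both events call their parent item logic first.
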(event EventBeginPlay
  (|CallParentFunction) ; This node is disabled and will not be called.\nDrag off pins to build functionality.
)

(event Collision|EventActorBeginOverlap
  (params (OtherActor :type Actor%20Object%20Reference)))

(event EventTick
  (params (DeltaSeconds :type Float%20%28single-precision%29))
  (|CallParentFunction DeltaSeconds) ; This node is disabled and will not be called.\nDrag off pins to build functionality.
)

(event EventItemHasInteracted
  (|CallParentFunction)
  (Collision|SetCollisionEnabled (Variables|Default|GetSphere) "NoCollision"))

(event EventUseItem
  (|CallParentFunction)
  (bind _asals_player_shooter_character_bp (Utilities|Casting|CastToALS_Player_ShooterCharacterBP (Game|Player|GetPlayerPawn 0)))
  (Default|PickedUpHealth _asals_player_shooter_character_bp 1e+02)
  (Audio|PlaySound2D "/Game/Sound/Misc/heal01.heal01"))

(fn ConstructionScript
  (|CallParentFunction))