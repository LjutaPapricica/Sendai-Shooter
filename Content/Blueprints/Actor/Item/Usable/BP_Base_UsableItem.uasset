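; Base actor for usable pickup items, with an empty UseItem function.
; A trigger overlap with the player pawn toggles the pawn's pickup message and shows or removes the item-name widget, which Tick positions above the mesh.
; On interaction, the item plays a pickup sound, hides itself, disables trigger collision and passes itself to the player's inventory rather than being destroyed.
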(event OnComponentBeginOverlap(Trigger)
  (params (OverlappedComponent :type Primitive%20Component%20Object%20Reference) (OtherActor :type Actor%20Object%20Reference) (OtherComp :type Primitive%20Component%20Object%20Reference) (OtherBodyIndex :type Integer) (bFromSweep :type Boolean) (SweepResult :type Hit%20Result%20Structure%20%28by%20ref%29))
  ;[1 1 1] overlap
  (CallFunction|PlayerIntoTrigger OtherActor true))

(event OnComponentEndOverlap(Trigger)
  (params (OverlappedComponent :type Primitive%20Component%20Object%20Reference) (OtherActor :type Actor%20Object%20Reference) (OtherComp :type Primitive%20Component%20Object%20Reference) (OtherBodyIndex :type Integer))
  ;[1 1 1] overlap
  (CallFunction|PlayerIntoTrigger OtherActor false))

(event EventBeginPlay
  ;[1 1 1] begin play
  (bind _returnvalue (UserInterface|CreateWidget "/Game/Blueprints/UI/BPUI_PickUpText.BPUI_PickUpText_C" 0 (Variables|Default|GetItemName)))
  (Variables|Default|SetPickUpUI _returnvalue))

(event EventTick
  (params (DeltaSeconds :type Float%20%28single-precision%29))
  ;[1 1 1] tick
  (if (Variables|Default|GetPlayerisinRange)
    (Default|PopUpTexttoWorldSpace (Variables|Default|GetPickUpUI) (+ (Transformation|GetWorldLocation (Variables|Default|GetMesh)) "0, 0,50.000000"))))

(event EventItemHasInteracted
  (Audio|PlaySound2D "/Game/Sound/PickUp_Cue.PickUp_Cue")
  (Rendering|SetActorHiddenInGame true)
  (Collision|SetCollisionEnabled (Variables|Default|GetTrigger) "NoCollision")
  (Default|CSetItemInfo (Variables|/Game/AdvancedLocomotionV2/Blueprints/ALS_Shooter/ALS_Player_ShooterCharacterBP.ALS_Player_ShooterCharacterBP_C|GetInventory (.AsALS%20Player%20Shooter%20Character%20BP (Utilities|Casting|CastToALS_Player_ShooterCharacterBP (Game|Player|GetPlayerPawn 0)))) self))

(fn ConstructionScript)

(fn PlayerIntoTrigger
  (params (TriggerdActor :type Object%20Object%20Reference) (Entered? :type Boolean))
  (bind _pickupui (Variables|Default|GetPickUpUI))
  (if (== TriggerdActor (Game|Player|GetPlayerPawn 0))
    (bind _output_get (Variables|Default|SetPlayerisinRange Entered?))
    (Class|BPIInteract|SetCanPickUp(Message) TriggerdActor _output_get)
    (if (Variables|Default|GetPlayerisinRange)
      (UserInterface|Viewport|AddtoViewport _pickupui 0)
      (else
        (Widget|RemovefromParent _pickupui)))))

(fn UseItem)