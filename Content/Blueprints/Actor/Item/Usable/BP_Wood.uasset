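; BP_Wood is a usable wood item that, when used, reappears at a hardcoded spot in the level.
; It extends a parent item class, adding a mesh collision disable after the parent's interaction handling.
; Using it applies a fixed world transform with rotation and stretched scale, unhides the actor and restores query-only mesh collision.
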(event EventBeginPlay
  (|CallParentFunction))

(event Collision|EventActorBeginOverlap
  (params (OtherActor :type Actor%20Object%20Reference)))

(event EventTick
  (params (DeltaSeconds :type Float%20%28single-precision%29))
  (|CallParentFunction DeltaSeconds) ; This node is disabled and will not be called.\nDrag off pins to build functionality.
)

(event EventUseItem
  (Transformation|SetActorTransform (Math|Transform|MakeTransform "1018.000000,-1300.000000,795.000000" "0,60.000000, 0" "1,2.000000,1"))
  (Rendering|SetActorHiddenInGame false)
  (Collision|SetCollisionEnabled (Variables|Character|GetMesh) "QueryOnly"))

(event EventItemHasInteracted
  (|CallParentFunction)
  (Collision|SetCollisionEnabled (Variables|Character|GetMesh) "NoCollision"))

(fn ConstructionScript
  (|CallParentFunction))