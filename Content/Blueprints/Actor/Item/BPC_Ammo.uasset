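; An ammo pickup item that refills the player's active weapon when it is picked up.
; On the HasPickedup event it casts player pawn 0 to ALS_Player_CharacterBP and gets the weapon at WeaponActiveIndex.
; It passes its minimum and maximum pickup amounts to that weapon's PickedUpAmmo, then destroys itself.
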(event EventBeginPlay
  (|CallParentFunction))

(event Collision|EventActorBeginOverlap
  (params (OtherActor :type Actor%20Object%20Reference))
  (|CallParentFunction OtherActor))

(event EventTick
  (params (DeltaSeconds :type Float%20%28single-precision%29))
  (|CallParentFunction DeltaSeconds))

(event EventHasPickedup
  (bind _returnvalue (Game|Player|GetPlayerPawn 0))
  (bind _asals_player_character_bp (Utilities|Casting|CastToALS_Player_CharacterBP _returnvalue))
  (Default|PickedUpAmmo (Utilities|Array|Get(acopy) (Variables|/Game/AdvancedLocomotionV2/Blueprints/ALS_Shooter/ALS_Player_CharacterBP.ALS_Player_CharacterBP_C|GetWeapons _asals_player_character_bp) (Variables|/Game/AdvancedLocomotionV2/Blueprints/ALS_Shooter/ALS_Player_CharacterBP.ALS_Player_CharacterBP_C|GetWeaponActiveIndex _asals_player_character_bp)) (Variables|Default|GetMin_CanPickedUp) (Variables|Default|GetMax_CanPickedUp))
  (Actor|DestroyActor))

(fn ConstructionScript
  (|CallParentFunction))