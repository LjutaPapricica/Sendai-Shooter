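; BPC_Ammo is an ammo pickup actor that resupplies the player's active weapon.
; On pickup, it runs the parent logic, casts player pawn 0 to ALS_Player_ShooterCharacterBP and calls PickUpAmmo on the NWeapons entry at WeaponActiveIndex.
; It then destroys itself.
; BeginPlay, Tick and the construction script only call their parent versions.
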(event EventBeginPlay
  (|CallParentFunction))

(event EventHasPickedup
  (bind _returnvalue (Game|Player|GetPlayerPawn 0))
  (bind _asals_player_shooter_character_bp (Utilities|Casting|CastToALS_Player_ShooterCharacterBP _returnvalue))
  (|CallParentFunction)
  (Default|PickUpAmmo (Utilities|Array|Get(acopy) (Variables|/Game/AdvancedLocomotionV2/Blueprints/ALS_Shooter/ALS_Player_ShooterCharacterBP.ALS_Player_ShooterCharacterBP_C|Getn_Weapons _asals_player_shooter_character_bp) (Variables|/Game/AdvancedLocomotionV2/Blueprints/ALS_Shooter/ALS_Player_ShooterCharacterBP.ALS_Player_ShooterCharacterBP_C|GetWeaponActiveIndex _asals_player_shooter_character_bp)))
  (Actor|DestroyActor))

(event EventTick
  (params (DeltaSeconds :type Float%20%28single-precision%29))
  (|CallParentFunction DeltaSeconds))

(fn ConstructionScript
  (|CallParentFunction))