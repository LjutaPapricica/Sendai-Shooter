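; Third-person player shooter character with movement, sprint and crouch timelines, damage-driven ragdoll death and item pickup.
; Input drives a two-slot weapon system with montage-based equipping, hold or toggle aiming, timer-repeated fire and reloading.
; Tick updates walk speed, bullet spread, rotation, trace-based foot IK fed to ABP_Shooter, aim-time autofocus depth of field and a muzzle-traced HUD position.
; The camera-switch timeline and its toggle are unwired.
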(event Input|ActionEvents|InputActionSprint
  (params (Key :type Key%20Structure))
  (bind _sprint (Variables|Default|GetSprint))
  (:Pressed
    (if (Variables|Movement|GetisAiming?)
      (Utilities|FlowControl|Sequence
        (:then_0
          (CallFunction|CUnEquipforSprint))
        (:then_1
          (Audio|Components|Audio|Play _sprint :!label _label)))
      (else
        (goto _label))))
  (:Released
    (Utilities|String|Reverse _sprint)))

(event Input|ActionEvents|InputActionCrouch
  (params (Key :type Key%20Structure))
  (bind _crouch (Variables|Default|GetCrouch))
  (:Pressed
    (Utilities|FlowControl|FlipFlop
      (:A
        (Variables|Default|SetisCrouching true)
        (Audio|Components|Audio|Play _crouch))
      (:B
        (Variables|Default|SetisCrouching false)
        (Utilities|String|Reverse _crouch)))))

(event Input|AxisEvents|InputAxisMoveForward
  (params (AxisValue :type Float%20%28single-precision%29))
  (Pawn|Input|AddMovementInput (Math|Vector|GetForwardVector (Math|Rotator|MakeRotator 0.0 0.0 (.Yaw (Math|Rotator|BreakRotator (Pawn|GetControlRotation :!class /Script/Engine.Pawn))))) AxisValue false))

(event Input|AxisEvents|InputAxisMoveRight
  (params (AxisValue :type Float%20%28single-precision%29))
  (Pawn|Input|AddMovementInput (Math|Vector|GetRightVector (Math|Rotator|MakeRotator 0.0 0.0 (.Yaw (Math|Rotator|BreakRotator (Pawn|GetControlRotation :!class /Script/Engine.Pawn))))) AxisValue false))

(event Input|AxisEvents|InputAxisTurn
  (params (AxisValue :type Float%20%28single-precision%29))
  (Pawn|Input|AddControllerYawInput AxisValue))

(event Input|AxisEvents|InputAxisLookUp
  (params (AxisValue :type Float%20%28single-precision%29))
  (Pawn|Input|AddControllerPitchInput (* -1 AxisValue)))

(event EventTick
  (params (DeltaSeconds :type Float%20%28single-precision%29))
  (Utilities|FlowControl|Sequence
    (:then_0
      (|SetMaxWalkSpeed))
    (:then_1
      (|CalculateBulletSpread))
    (:then_2
      (|SetisMoving))
    (:then_3
      (|SetOrientRotFromisMoving))
    (:then_4
      (CallFunction|FootIK))
    (:then_5
      (|TickAutoFocus))
    (:then_6
      (|SetHUDLocation))))

(event EventBeginPlay
  (Utilities|FlowControl|Sequence
    (:then_0
      (Variables|Movement|SetCurrentSpeed (Variables|Movement|GetInitialSpeed)))
    (:then_1
      (Variables|Animation|SetTPSAnimRefe (Components|SkeletalMesh|GetAnimInstance (Variables|Character|GetMesh))))))

(event Game|Damage|EventAnyDamage
  (params (Damage :type Float%20%28single-precision%29) (DamageType :type Damage%20Type%20Object%20Reference) (InstigatedBy :type Controller%20Object%20Reference) (DamageCauser :type Actor%20Object%20Reference))
  (bind _output_get (Variables|State|SetHP (Math|Float|Clamp(Float) (- (Variables|State|GetHP) Damage) 0.0 1e+02)))
  (if (<= _output_get 0.0)
    (Physics|SetSimulatePhysics (Variables|Character|GetMesh) true)
    (Pawn|Components|CharacterMovement|DisableMovement (Variables|Character|GetCharacterMovement))))

(event Input|ActionEvents|InputActionInteract
  (params (Key :type Key%20Structure))
  ;[0 0 0] Weapon Interact
  (:Pressed
    (bind _asbps_weapon (Utilities|Casting|CastToBPS_Weapon (Utilities|Array|Get(acopy) (Collision|GetOverlappingActors (Variables|Collision|GetCapsuleComponent) "/Game/Blueprints/Actor/Weapon/BPS_Weapon.BPS_Weapon_C" :!class /Script/Engine.PrimitiveComponent)))
      (:then
        (if (< (Variables|Weapon|GetWeaponIndex) 2)
          (bind _output_get (Variables|Weapon|SetInteractedWeapon _asbps_weapon))
          (Utilities|Array|SetArrayElem (Variables|Weapon|GetWeapons) (Variables|Weapon|GetWeaponIndex) _output_get true)
          (if (and (!= (Variables|Weapon|GetInteractedWeapon) 0) (Utilities|DoesObjectImplementInterface (Variables|Weapon|GetInteractedWeapon) "/Game/Blueprints/UI/BPI_Interact.BPI_Interact_C"))
            (Class|BPIInteract|WeaponHasInteracted(Message) (Variables|Weapon|GetInteractedWeapon) (Variables|Character|GetMesh) "None" (Utilities|Array|Get(acopy) (Variables|Weapon|GetSockets) (Variables|Weapon|GetWeaponIndex)))
            (Math|Integer|IncrementInt (Variables|Weapon|GetWeaponIndex)))
          (else
            (Development|PrintString "Full of Slot !"))))
      (:CastFailed
        (bind _asbps_item (Utilities|Casting|CastToBPS_Item (Utilities|Array|Get(acopy) (Collision|GetOverlappingActors (Variables|Collision|GetCapsuleComponent) "/Game/Blueprints/Actor/Item/BPS_Item.BPS_Item_C" :!class /Script/Engine.PrimitiveComponent))))
        (Class|BPIInteract|ItemHasInteracted(Message) _asbps_item)))))

(event Custom|c_Equip%20/%20UnEquip
  (bind _weapons (Variables|Weapon|GetWeapons))
  (bind _weaponseletindex (Variables|Weapon|GetWeaponSeletIndex))
  (bind _output (Utilities|Array|Get(acopy) _weapons _weaponseletindex))
  ;[0 1 0.9705] Equip / UnEquip
  (if (Variables|Movement|GetisAiming?)
    (Default|EquipWeapon _output (Variables|Character|GetMesh))
    (Variables|Weapon|SetEquipedWeapon _output)
    (Variables|Weapon|SetPrevWeaponIndex (Variables|Weapon|GetWeaponSeletIndex))
    (else
      (Default|EquipWeapon (Variables|Weapon|GetEquipedWeapon) (Variables|Character|GetMesh))
      (Variables|Weapon|SetEquipedWeapon 0))))

(event Custom|c_Fire
  ;[0 0 0] Fire Weapon
  (bind _equipedweapon (Variables|Weapon|GetEquipedWeapon)
    (:then
      (Default|CFire _equipedweapon (Variables|Animation|GetTPSAnimRefe) (Variables|Weapon|GetSpreadCurrent) self)
      (Variables|Weapon|SetBulletHitLoc (Variables|/Game/Blueprints/Actor/Weapon/BPS_Weapon.BPS_Weapon_C|GetHitLoc _equipedweapon))
      (CallFunction|IncreaseSpread 0.0))
    (:else)))

(event Custom|c_InstantUnEquip
  ;[0 1 0.9705] Equip / UnEquip
  (Animation|Montage|MontagePlay (Variables|Animation|GetTPSAnimRefe) "/Game/Animations/Grayman/Montage/Mont_EquipWeapon.Mont_EquipWeapon" 1.0 "MontageLength" 0.0)
  (CallFunction|CRemoveHUD)
  (Default|EquipWeapon (Variables|Weapon|GetEquipedWeapon) (Variables|Character|GetMesh))
  (Variables|Weapon|SetEquipedWeapon 0))

(event Custom|c_RemoveHUD
  ;[1 0 0] Aim
  (Widget|RemovefromParent (Variables|Default|GetUI_HUD))
  (Variables|/Script/Engine.CharacterMovementComponent|SetbOrientRotationToMovement (Variables|Character|GetCharacterMovement) true))

(event Custom|c_AddHUD
  ;[1 0 0] Aim
  (bind _returnvalue (UserInterface|CreateWidget "/Game/Blueprints/UI/BPUI_HUD.BPUI_HUD_C" 0 0))
  (bind _output_get (Variables|Default|SetUI_HUD _returnvalue))
  (UserInterface|Viewport|AddtoViewport _output_get 0))

(event Custom|c_InstantEquip
  (bind _weapons (Variables|Weapon|GetWeapons))
  (bind _weaponseletindex (Variables|Weapon|GetWeaponSeletIndex))
  (bind _output (Utilities|Array|Get(acopy) _weapons _weaponseletindex))
  ;[0 1 0.9705] Equip / UnEquip
  (CallFunction|CAddHUD)
  (Default|EquipWeapon _output (Variables|Character|GetMesh))
  (Variables|Weapon|SetEquipedWeapon _output)
  (Variables|Weapon|SetPrevWeaponIndex (Variables|Weapon|GetWeaponSeletIndex)))

(event Custom|c_UnEquipForSprint
  (bind _tpsanimrefe (Variables|Animation|GetTPSAnimRefe))
  (bind _aiming (Variables|Default|GetAiming))
  ;[1 0 0] Aim
  (if (Variables|Input|GetToggleAim?)
    (Utilities|FlowControl|FlipFlop
      (:A
        (Animation|Montage|MontagePlay _tpsanimrefe "/Game/Animations/Grayman/Montage/Mont_EquipWeapon.Mont_EquipWeapon" 1.0 "MontageLength" 0.0 :!label _label)
        (Variables|Movement|SetisAiming? true)
        (Audio|Components|Audio|Play _aiming)
        (bind _returnvalue (UserInterface|CreateWidget "/Game/Blueprints/UI/BPUI_HUD.BPUI_HUD_C" 0 0))
        (bind _output_get (Variables|Default|SetUI_HUD _returnvalue))
        (UserInterface|Viewport|AddtoViewport _output_get 0))
      (:B
        (Animation|Montage|MontagePlay _tpsanimrefe "/Game/Animations/Grayman/Montage/Mont_EquipWeapon.Mont_EquipWeapon" 1.0 "MontageLength" 0.0)
        (Variables|Movement|SetisAiming? false)
        (Utilities|String|Reverse _aiming)
        (Widget|RemovefromParent (Variables|Default|GetUI_HUD))
        (Variables|/Script/Engine.CharacterMovementComponent|SetbOrientRotationToMovement (Variables|Character|GetCharacterMovement) true)))
    (else
      (goto _label))))

(event Input|ActionEvents|InputActionAim
  (params (Key :type Key%20Structure))
  (bind _interactedweapon (Variables|Weapon|GetInteractedWeapon))
  (bind _tpsanimrefe (Variables|Animation|GetTPSAnimRefe))
  (bind _aiming (Variables|Default|GetAiming))
  (bind _toggleaim_ (Variables|Input|GetToggleAim?))
  ;[1 0 0] Aim
  (:Pressed
    (if (!= _interactedweapon 0)
      (if _toggleaim_
        (Utilities|FlowControl|FlipFlop
          (:A
            (Animation|Montage|MontagePlay _tpsanimrefe "/Game/Animations/Grayman/Montage/Mont_EquipWeapon.Mont_EquipWeapon" 1.0 "MontageLength" 0.0 :!label _label)
            (Variables|Movement|SetisAiming? true)
            (Audio|Components|Audio|Play _aiming)
            (bind _returnvalue (UserInterface|CreateWidget "/Game/Blueprints/UI/BPUI_HUD.BPUI_HUD_C" 0 0))
            (bind _output_get (Variables|Default|SetUI_HUD _returnvalue))
            (UserInterface|Viewport|AddtoViewport _output_get 0))
          (:B
            (Animation|Montage|MontagePlay _tpsanimrefe "/Game/Animations/Grayman/Montage/Mont_EquipWeapon.Mont_EquipWeapon" 1.0 "MontageLength" 0.0 :!label _label_2)
            (Variables|Movement|SetisAiming? false)
            (Utilities|String|Reverse _aiming)
            (Widget|RemovefromParent (Variables|Default|GetUI_HUD))
            (Variables|/Script/Engine.CharacterMovementComponent|SetbOrientRotationToMovement (Variables|Character|GetCharacterMovement) true)))
        (else
          (goto _label)))))
  (:Released
    (if (!= _interactedweapon 0)
      (if (not _toggleaim_)
        (goto _label_2)))))

(event Input|ActionEvents|InputActionChangeCamera
  (params (Key :type Key%20Structure)))

(event Input|ActionEvents|InputActionReload
  (params (Key :type Key%20Structure))
  (bind _equipedweapon (Variables|Weapon|GetEquipedWeapon))
  ;[1 1 1] Reload
  (:Pressed
    (if (!= _equipedweapon 0)
      (Default|CReload _equipedweapon (Variables|Animation|GetTPSAnimRefe)))))

(event Input|ActionEvents|InputActionFire
  (params (Key :type Key%20Structure))
  ;[0 0 0] Fire Weapon
  (:Pressed
    (if (!= (Variables|Weapon|GetInteractedWeapon) 0)
      (CallFunction|CFire)
      (Utilities|Time|SetTimerbyFunctionName 0 "c_Fire" (/ 1.0 (Variables|/Game/Blueprints/Actor/Weapon/BPS_Weapon.BPS_Weapon_C|GetFireRate (Variables|Weapon|GetEquipedWeapon))) true)))
  (:Released
    (Utilities|Time|ClearTimerbyFunctionName 0 "c_Fire")))

(event Input|ActionEvents|InputActionEquipMain
  (params (Key :type Key%20Structure))
  ;[0.8875 1 0] Equip Weapon / Hot key 1,2
  (:Pressed
    (Variables|Weapon|SetWeaponSeletIndex 0)
    (if (and (Variables|Movement|GetisAiming?) (!= (Variables|Weapon|GetWeaponSeletIndex) (Variables|Weapon|GetPrevWeaponIndex)))
      (CallFunction|CInstantUnEquip)
      (Utilities|FlowControl|Delay 1.0)
      (CallFunction|CInstantEquip))))

(event Input|ActionEvents|InputActionEquipSub
  (params (Key :type Key%20Structure))
  ;[0.8875 1 0] Equip Weapon / Hot key 1,2
  (:Pressed
    (Variables|Weapon|SetWeaponSeletIndex 1)
    (if (and (Variables|Movement|GetisAiming?) (!= (Variables|Weapon|GetWeaponSeletIndex) (Variables|Weapon|GetPrevWeaponIndex)))
      (CallFunction|CInstantUnEquip)
      (Utilities|FlowControl|Delay 1.0)
      (CallFunction|CInstantEquip))))

(fn ConstructionScript)

(fn IncreaseSpread
  (params (Increase%20Spread :type Float%20%28single-precision%29))
  (if (>= (+ Increase%20Spread (Variables|Weapon|GetSpreadCurrent)) (Variables|Weapon|GetSpreadMax))
    (Variables|Weapon|SetSpreadCurrent (Variables|Weapon|GetSpreadMax))
    (else
      (Variables|Weapon|SetSpreadCurrent (+ Increase%20Spread (Variables|Weapon|GetSpreadCurrent))))))

(fn DecreaseSpread
  (params (Decrease%20Amount :type Float%20%28single-precision%29))
  (if (<= (- (Variables|Weapon|GetSpreadCurrent) Decrease%20Amount) (Variables|Weapon|GetSpreadMin))
    (Variables|Weapon|SetSpreadCurrent (Variables|Weapon|GetSpreadMin))
    (else
      (Variables|Weapon|SetSpreadCurrent (- (Variables|Weapon|GetSpreadCurrent) Decrease%20Amount)))))

(fn IKFootTrace
  (params (Socket%20Name :type Name) (Trace%20Distance :type Float%20%28single-precision%29))
  (bind _returnvalue (Transformation|GetActorLocation))
  (bind _mesh (Variables|Character|GetMesh))
  (bind _capsulecomponent (Variables|Collision|GetCapsuleComponent))
  (bind _returnvalue_2 (Transformation|GetSocketLocation _mesh Socket%20Name))
  (bind _z (Math|Vector|BreakVector _returnvalue))
  (bind _capsulehalfheight (Variables|/Script/Engine.CapsuleComponent|GetCapsuleHalfHeight _capsulecomponent))
  (bind (_x _y) (Math|Vector|BreakVector _returnvalue_2))
  (bind (_outhit _returnvalue_3) (Collision|LineTraceByChannel (Math|Vector|MakeVector _x _y (- _z (/ _capsulehalfheight 2.0))) (Math|Vector|MakeVector _x _y (- _z Trace%20Distance)) "TraceTypeQuery1" false (Utilities|Array|MakeArray (Components|GetOwner (Variables|Collision|GetCapsuleComponent))) "None"))
  (return _returnvalue_3 (Math|Float|SelectFloat (/ (- (- _z _capsulehalfheight) (.Z (Math|Vector|BreakVector (.ImpactPoint (Collision|BreakHitResult _outhit))))) -1.0) 0.0 _returnvalue_3) (.ImpactPoint (Collision|BreakHitResult _outhit))))

(fn FootIK
  (bind _asabp_shooter (Utilities|Casting|CastToABP_Shooter (Variables|Animation|GetTPSAnimRefe)))
  (LocalVariables|SetAnimBPRefe _asabp_shooter)
  (Utilities|FlowControl|Sequence
    (:then_0
      (bind (_hit _hip_offset _effector_location) (CallFunction|IKFootTrace "RightFootSocket" 1.5e+02))
      (bind _output_get (Variables|/Game/Blueprints/Pawn/Player/ABP_Shooter.ABP_Shooter_C|SetRightEffector (LocalVariables|GetAnimBPRefe) (+ _effector_location "0, 0,15.000000")))
      (if _hit
        (if (>= (Variables|/Game/Blueprints/Pawn/Player/ABP_Shooter.ABP_Shooter_C|GetSpeed (LocalVariables|GetAnimBPRefe)) 15.0)
          (bind _output_get_2 (Variables|/Game/Blueprints/Pawn/Player/ABP_Shooter.ABP_Shooter_C|SetIKAlphaRight (LocalVariables|GetAnimBPRefe) (/ (+ (Math|Float|Clamp(Float) (- 1.0 (/ (Math|Vector|VectorLength (- (Transformation|GetSocketLocation (Variables|Character|GetMesh) "RightFootSocket") _output_get)) 34.0)) 0.0 0.61) (Variables|Animation|GetOldAlphaRight)) 2.0)))
          (Variables|Animation|SetOldAlphaRight _output_get_2)
          (else
            (Variables|/Game/Blueprints/Pawn/Player/ABP_Shooter.ABP_Shooter_C|SetIKAlphaRight (LocalVariables|GetAnimBPRefe) 0.85)))
        (else
          (Variables|/Game/Blueprints/Pawn/Player/ABP_Shooter.ABP_Shooter_C|SetIKAlphaRight (LocalVariables|GetAnimBPRefe) 0.0))))
    (:then_1
      (bind (_hit_2 _hip_offset_2 _effector_location_2) (CallFunction|IKFootTrace "LeftFootSocket" 1.5e+02))
      (bind _output_get_3 (Variables|/Game/Blueprints/Pawn/Player/ABP_Shooter.ABP_Shooter_C|SetLeftEffector (LocalVariables|GetAnimBPRefe) (+ _effector_location_2 "0, 0,15.000000")))
      (if _hit_2
        (if (>= (Variables|/Game/Blueprints/Pawn/Player/ABP_Shooter.ABP_Shooter_C|GetSpeed (LocalVariables|GetAnimBPRefe)) 15.0)
          (bind _output_get_4 (Variables|/Game/Blueprints/Pawn/Player/ABP_Shooter.ABP_Shooter_C|SetIKAlphaLeft (LocalVariables|GetAnimBPRefe) (/ (+ (Variables|Animation|GetOldAlphaLeft) (Math|Float|Clamp(Float) (- 1.0 (/ (Math|Vector|VectorLength (- (Transformation|GetSocketLocation (Variables|Character|GetMesh) "LeftFootSocket") _output_get_3)) 34.0)) 0.0 0.61)) 2.0)))
          (Variables|Animation|SetOldAlphaLeft _output_get_4)
          (if (>= (Math|Float|Absolute(Float) _hip_offset) (Math|Float|Absolute(Float) _hip_offset_2))
            (Variables|/Game/Blueprints/Pawn/Player/ABP_Shooter.ABP_Shooter_C|SetHipOffset (LocalVariables|GetAnimBPRefe) _hip_offset)
            (else
              (Variables|/Game/Blueprints/Pawn/Player/ABP_Shooter.ABP_Shooter_C|SetHipOffset (LocalVariables|GetAnimBPRefe) _hip_offset_2)))
          (else
            (Variables|/Game/Blueprints/Pawn/Player/ABP_Shooter.ABP_Shooter_C|SetIKAlphaLeft (LocalVariables|GetAnimBPRefe) 0.85)))
        (else
          (Variables|/Game/Blueprints/Pawn/Player/ABP_Shooter.ABP_Shooter_C|SetIKAlphaLeft (LocalVariables|GetAnimBPRefe) 0.0))))))

(fn AutoFocus
  (bind _returnvalue (Game|GetPlayerCameraManager 0))
  (bind _returnvalue_2 (Transformation|GetActorLocation _returnvalue))
  (bind (_outhit _returnvalue_3) (Collision|LineTraceByChannel _returnvalue_2 (+ _returnvalue_2 (* (Math|Vector|GetForwardVector (Transformation|GetActorRotation _returnvalue)) 1e+04)) "TraceTypeQuery1" false 0 "None"))
  (if _returnvalue_3
    (LocalVariables|SetFocusLoc (Math|Vector|VectorLength (- (.ImpactPoint (Collision|BreakHitResult _outhit)) _returnvalue_2)))
    (else
      (LocalVariables|SetFocusLoc (Variables|/Script/Engine.SpringArmComponent|GetTargetArmLength (Variables|Default|GetTPSSpringArm)))))
  (Variables|/Script/Engine.CameraComponent|SetPostProcessSettings (Variables|Default|GetTPSCamera) (Utilities|Struct|MakePostProcessSettings "DOFM_CircleDOF" 1.0 (LocalVariables|GetFocusLoc) 1e+02 1e+02 1e+02)))