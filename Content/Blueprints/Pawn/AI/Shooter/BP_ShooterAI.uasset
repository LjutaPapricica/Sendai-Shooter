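; AI shooter pawn that carries a sci-fi rifle, tracks perceived actors and drives its aim animation.
; BeginPlay spawns the rifle on a hand-holder socket and caches the anim instance.
; Perception updates store a sensed non-shooter actor in SawActor, clearing it when sensing fails.
; Custom events, not called here, start aiming and interpolate pitch/yaw toward a target, messaging the anim instance and debug-printing the angles.
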(event OnPerceptionUpdated(AIPerception)
  (params (UpdatedActors :type Array%20of%20Actor%20Object%20References))
  (for _array_element UpdatedActors
    (bind _info (Class|AIPerceptionComponent|GetActorsPerception (Variables|Default|GetAIPerception) _array_element))
    (if (.bSuccessfullySensed (Utilities|Struct|BreakAIStimulus (Utilities|Array|Get(acopy) (.LastSensedStimuli (Utilities|Struct|BreakActorPerceptionBlueprintInfo _info)))))
      (if (not (.bSuccess (Utilities|Casting|CastToBP_ShooterAI (.Target (Utilities|Struct|BreakActorPerceptionBlueprintInfo _info)))))
        (Variables|Sensed|SetSawActor (.Target (Utilities|Struct|BreakActorPerceptionBlueprintInfo _info))))
      (else
        (Variables|Sensed|SetSawActor 0)))))

(event EventBeginPlay
  (Utilities|FlowControl|Sequence
    (:then_0
      (bind _returnvalue (Game|SpawnActorfromClass "/Game/Blueprints/Actor/Weapon/BPC_ScifiRifle.BPC_ScifiRifle_C" (Math|Transform|MakeTransform "0, 0, 0") "AlwaysSpawn" 0 0))
      (Class|BPIInteract|WeaponHasInteracted(Message) _returnvalue (Variables|Character|GetMesh) "WeaponHolder_01"))
    (:then_1
      (Variables|Animation|SetAnimInst (Components|SkeletalMesh|GetAnimInstance (Variables|Character|GetMesh))))))

(event Custom|c_StartAim
  (Variables|Animation|SetisAiming? true)
  (Class|BPIAIMovement|SetIsAiming(Message) (Variables|Animation|GetAnimInst) true))

(event Custom|c_SetPitch%20/%20Yaw
  (params (TargetActor :type Actor%20Object%20Reference))
  (Variables|Animation|SetPitch (.Pitch (Math|Rotator|BreakRotator (Math|Interpolation|RInterpTo (Math|Rotator|MakeRotator 0.0 (Variables|Animation|GetPitch) (Variables|Animation|GetYaw)) (Math|Rotator|FindLookatRotation (Transformation|GetActorLocation) (Transformation|GetActorLocation TargetActor)) (Utilities|Time|GetWorldDeltaSeconds) 1e+03))))
  (Variables|Animation|SetYaw (.Yaw (Math|Rotator|BreakRotator (Math|Interpolation|RInterpTo (Math|Rotator|MakeRotator 0.0 (Variables|Animation|GetPitch) (Variables|Animation|GetYaw)) (Math|Rotator|FindLookatRotation (Transformation|GetActorLocation) (Transformation|GetActorLocation TargetActor)) (Utilities|Time|GetWorldDeltaSeconds) 1e+03))))
  (Class|BPIAIMovement|SetPitch/Yaw(Message) (Variables|Animation|GetAnimInst) (Variables|Animation|GetPitch) (Variables|Animation|GetYaw))
  (Development|PrintString (Utilities|String|Append "Pitch : " (Utilities|String|ToString(Float) (Variables|Animation|GetPitch)) " " "Yaw : " (Utilities|String|ToString(Float) (Variables|Animation|GetYaw)))))

(fn ConstructionScript)