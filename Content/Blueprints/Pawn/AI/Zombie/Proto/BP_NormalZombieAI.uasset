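; Prototype normal zombie pawn that takes damage, reddens as it is hurt and ragdolls when its health runs out.
; AnyDamage lowers clamped HP, records the damage causer and shifts the body color toward red in proportion to the damage.
; The tint accumulates on a dynamic material instance created in the construction script.
; At zero HP, capsule collision and movement are disabled and the mesh simulates physics.
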(event Custom|c_ChangeBodyColor
  (params (Damage :type Float%20%28single-precision%29))
  (bind _returnvalue (/ Damage 1e+02))
  (bind _mi_body (Variables|Default|GetMI_Body))
  ;[1 0.4062 0.4062] Change body color
  (bind _returnvalue_2 (Rendering|Material|GetVectorParameterValue _mi_body "BodyColor" :!class /Script/Engine.MaterialInstanceDynamic))
  (Rendering|Material|SetVectorParameterValue _mi_body "BodyColor" (Utilities|Struct|MakeLinearColor (Math|Float|Clamp(Float) (+ _returnvalue (.R (Utilities|Struct|BreakLinearColor _returnvalue_2)))) (Math|Float|Clamp(Float) (- (.G (Utilities|Struct|BreakLinearColor _returnvalue_2)) _returnvalue)) (Math|Float|Clamp(Float) (- (.B (Utilities|Struct|BreakLinearColor _returnvalue_2)) _returnvalue)) (.A (Utilities|Struct|BreakLinearColor _returnvalue_2))) :!class /Script/Engine.MaterialInstanceDynamic))

(event Game|Damage|EventAnyDamage
  (params (Damage :type Float%20%28single-precision%29) (DamageType :type Damage%20Type%20Object%20Reference) (InstigatedBy :type Controller%20Object%20Reference) (DamageCauser :type Actor%20Object%20Reference))
  (Variables|Default|SetHP (Math|Float|Clamp(Float) (- (Variables|Default|GetHP) Damage) 0.0 1e+02))
  (Variables|Default|SetDamageCause DamageCauser)
  (CallFunction|CChangeBodyColor Damage)
  (if (<= (Variables|Default|GetHP) 0.0)
    (Collision|SetCollisionEnabled (Variables|Collision|GetCapsuleComponent) "NoCollision")
    (Physics|SetSimulatePhysics (Variables|Character|GetMesh) true)
    (Pawn|Components|CharacterMovement|DisableMovement (Variables|Character|GetCharacterMovement))))

(fn ConstructionScript
  (bind _returnvalue (Rendering|Material|CreateDynamicMaterialInstance (Variables|Character|GetMesh) 0 0 :!class /Script/Engine.PrimitiveComponent))
  (Variables|Default|SetMI_Body _returnvalue))