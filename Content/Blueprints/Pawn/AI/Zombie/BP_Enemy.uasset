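; Zombie enemy character that chases the player, jumps to requested destinations and ragdolls when killed.
; A looping timer re-issues a move toward the player pawn while movement is allowed, with walk speed slightly randomized at spawn.
; DoJumpRequest pauses chasing and launches the character along a boosted projectile arc until landing re-enables it.
; Damage lowers clamped HP; at zero, the mesh simulates physics and capsule collision and movement are disabled.
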(event Custom|ChaseToPlayer
  (if (Variables|Default|GetCanMove)
    (AI|Navigation|SimpleMovetoActor (AI|GetAIController self) (Game|Player|GetPlayerPawn 0))))

(event EventBeginPlay
  (Utilities|FlowControl|Sequence
    (:then_0
      (Utilities|Time|SetTimerbyFunctionName 0 "ChaseToPlayer" 1.0 true))
    (:then_1
      (Variables|/Script/Engine.CharacterMovementComponent|SetMaxWalkSpeed (Variables|Character|GetCharacterMovement) (Math|Random|RandomFloatinRange 2.5e+02 3e+02)))))

(event EventOnLanded
  (params (Hit :type Hit%20Result%20Structure%20%28by%20ref%29))
  (Variables|Default|SetCanMove true))

(event Game|Damage|EventAnyDamage
  (params (Damage :type Float%20%28single-precision%29) (DamageType :type Damage%20Type%20Object%20Reference) (InstigatedBy :type Controller%20Object%20Reference) (DamageCauser :type Actor%20Object%20Reference))
  (bind _mesh (Variables|Character|GetMesh))
  (bind _output_get (Variables|Default|SetHP (Math|Float|Clamp(Float) (- (Variables|Default|GetHP) Damage))))
  (if (<= _output_get 0.0)
    (Collision|SetCollisionEnabled _mesh "PhysicsOnly")
    (Physics|SetSimulatePhysics _mesh true)
    (Collision|SetCollisionEnabled (Variables|Collision|GetCapsuleComponent) "NoCollision")
    (Pawn|Components|CharacterMovement|DisableMovement (Variables|Character|GetCharacterMovement))))

(fn ConstructionScript)

(fn DoJumpRequest
  (params (Destination :type Vector))
  (Variables|Default|SetCanMove false)
  (bind _outlaunchvelocity (Game|SuggestProjectileVelocityCustomArc (Transformation|GetActorLocation) Destination 0.0 0.5))
  (Character|LaunchCharacter (* _outlaunchvelocity 1.25) true true))