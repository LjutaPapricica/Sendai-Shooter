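; BP_AIDirector tracks registered zombie enemies and ends the game once all of them are dead.
; SetReference registers enemies, and a one-second looping timer runs CheckEnemyRemain, which counts the dead whenever CanCheck is set.
; When the count matches the list, a one-shot end event fades to black, shows the title widget, disables player input and removes the HUD, inventory and objective UI.
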(event Custom|c_EndGame
  (bind _returnvalue (Game|Player|GetPlayerPawn 0))
  (Utilities|FlowControl|DoOnce false
    (:Completed
      (CameraFades|StartCameraFade :self (Game|GetPlayerCameraManager 0) :ToAlpha 1.0 :Duration 3.0 :bHoldWhenFinished true)
      (Utilities|FlowControl|Delay 3.0)
      (Utilities|FlowControl|Sequence
        (:then_0
          (bind _returnvalue_2 (UserInterface|CreateWidget "/Game/Blueprints/UI/BPUI_Title.BPUI_Title_C"))
          (UserInterface|Viewport|AddtoViewport _returnvalue_2 0))
        (:then_1
          (Input|DisableInput _returnvalue (Game|GetPlayerController 0)))
        (:then_2
          (bind _asals_player_shooter_character_bp (Utilities|Casting|CastToALS_Player_ShooterCharacterBP _returnvalue))
          (Widget|RemovefromParent (Variables|/Game/AdvancedLocomotionV2/Blueprints/ALS_Shooter/ALS_Player_ShooterCharacterBP.ALS_Player_ShooterCharacterBP_C|GetHUD _asals_player_shooter_character_bp))
          (Default|CustomEvent0 _asals_player_shooter_character_bp))
        (:then_3
          (bind _outactors (Actor|GetAllActorsOfClass "/Game/Blueprints/Meta/Event/BP_EventHandler.BP_EventHandler_C"))
          (Widget|RemovefromParent (Variables|/Game/Blueprints/Meta/Event/BP_EventHandler.BP_EventHandler_C|GetUI_Objective (Utilities|Array|Get(acopy) _outactors))))))))

(event EventBeginPlay
  (Utilities|Time|SetTimerbyFunctionName 0 "CheckEnemyRemain" 1.0 true))

(fn ConstructionScript)

(fn CheckEnemyRemain
  (bind _enemies (Variables|Default|GetEnemies))
  (bind _returnvalue (Utilities|Array|Length _enemies))
  (if (Variables|Default|GetCanCheck)
    (for _array_element (Variables|Default|GetEnemies)
      (if (Variables|/Game/Blueprints/Pawn/AI/Zombie/BP_Enemy.BP_Enemy_C|GetDead _array_element)
        (Math|Integer|IncrementInt (Variables|Default|GetDeathCnt))))
    (Development|PrintString (Utilities|String|Append (Utilities|String|ToString(Integer) (Variables|Default|GetDeathCnt)) " : " (Utilities|String|ToString(Integer) _returnvalue)))
    (if (== (Variables|Default|GetDeathCnt) _returnvalue)
      (CallFunction|CEndGame)
      (else
        (Variables|Default|SetDeathCnt 0)))))

(fn SetReference
  (params (Reference :type BP%20Enemy%20Object%20Reference%20%28by%20ref%29))
  (if (Utilities|IsValid Reference)
    (Utilities|Array|Add (Variables|Default|GetEnemies) Reference)))