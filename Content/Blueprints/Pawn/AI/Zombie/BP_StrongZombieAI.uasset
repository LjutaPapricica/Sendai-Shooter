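; Strong zombie enemy pawn that hunts, melees and ragdolls on death.
; A timer pulses a growing detection sphere until it overlaps a non-zombie actor, which AI MoveTo then chases repeatedly; damage retargets to the causer.
; Player overlap on AttackablePoint messages the AnimBP, and AttackStart fires a forward fan of line traces to apply damage.
; Walk speed is randomly weighted at spawn, and hits redden the body material and loosen head physics.
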(event OnComponentBeginOverlap(SphereCollision)
  (params (OverlappedComponent :type Primitive%20Component%20Object%20Reference) (OtherActor :type Actor%20Object%20Reference) (OtherComp :type Primitive%20Component%20Object%20Reference) (OtherBodyIndex :type Integer) (bFromSweep :type Boolean) (SweepResult :type Hit%20Result%20Structure%20%28by%20ref%29))
  ;[1 0 0.5579] Set to value sensed actor when we overlapped with sphere collision
  (if (not (.bSuccess (Utilities|Casting|CastToBP_StrongZombieAI OtherActor)))
    (Utilities|FlowControl|DoOnce false
      (:Completed
        (Variables|Default|SetSensedActor OtherActor)
        (CallFunction|CTracetoSensedActor)))))

(event OnComponentBeginOverlap(AttackablePoint)
  (params (OverlappedComponent :type Primitive%20Component%20Object%20Reference) (OtherActor :type Actor%20Object%20Reference) (OtherComp :type Primitive%20Component%20Object%20Reference) (OtherBodyIndex :type Integer) (bFromSweep :type Boolean) (SweepResult :type Hit%20Result%20Structure%20%28by%20ref%29))
  (Utilities|Casting|CastToBP_ShooterCharacterGirl OtherActor)
  (Class|BPIAIMovement|Attack(Message) (Components|SkeletalMesh|GetAnimInstance (Variables|Character|GetMesh))))

(event Custom|c_SphereColScaleUp
  (bind _spherecollision (Variables|Default|GetSphereCollision))
  (bind _sphereradius (Variables|/Script/Engine.SphereComponent|GetSphereRadius _spherecollision))
  ;[0.3961 1 0.1739] Set sphere collision scale
  (if (== (Variables|Default|GetSensedActor) 0)
    (if (>= _sphereradius 2e+03)
      (Components|Sphere|SetSphereRadius _spherecollision 32.0 true)
      (else
        (Components|Sphere|SetSphereRadius _spherecollision (+ _sphereradius 5e+01) true)))))

(event Custom|c_TraceToSensedActor
  ;[0 0.8969 1] Move to sensed actor and send damage info overlapped actor
  (if (!= (Variables|Default|GetSensedActor) 0)
    (AI|AIMoveTo self "0, 0, 0" (Variables|Default|GetSensedActor) 5.0 false
      (:OnSuccess
        _)
      (:OnFail
        _))
    (CallFunction|CTracetoSensedActor)))

(event Custom|c_SetBodyColor
  (params (Damage :type Float%20%28single-precision%29))
  (bind _returnvalue (/ Damage 1e+02))
  (bind _mi_body (Variables|Default|GetMI_Body))
  ;[1 0 0] Take any damage and dead logic
  (bind _returnvalue_2 (Rendering|Material|GetVectorParameterValue _mi_body "BodyColor" :!class /Script/Engine.MaterialInstanceDynamic))
  (Rendering|Material|SetVectorParameterValue _mi_body "BodyColor" (Utilities|Struct|MakeLinearColor (Math|Float|Clamp(Float) (+ _returnvalue (.R (Utilities|Struct|BreakLinearColor _returnvalue_2)))) (Math|Float|Clamp(Float) (- (.G (Utilities|Struct|BreakLinearColor _returnvalue_2)) _returnvalue)) (Math|Float|Clamp(Float) (- (.B (Utilities|Struct|BreakLinearColor _returnvalue_2)) _returnvalue)) (.A (Utilities|Struct|BreakLinearColor _returnvalue_2))) :!class /Script/Engine.MaterialInstanceDynamic))

(event Game|Damage|EventAnyDamage
  (params (Damage :type Float%20%28single-precision%29) (DamageType :type Damage%20Type%20Object%20Reference) (InstigatedBy :type Controller%20Object%20Reference) (DamageCauser :type Actor%20Object%20Reference))
  (bind _mesh (Variables|Character|GetMesh))
  ;[1 0 0] Take any damage and dead logic
  (Class|SkeletalMeshComponent|SetAllBodiesBelowSimulatePhysics (Variables|Character|GetMesh) (Utilities|Name|MakeLiteralName "head") true true)
  (Variables|Default|SetHP (Math|Float|Clamp(Float) (- (Variables|Default|GetHP) Damage) 0.0 1e+02))
  (Variables|Default|SetSensedActor DamageCauser)
  (CallFunction|CSetBodyColor Damage)
  (Effects|SpawnEmitteratLocation "/Game/Imported/Effects/ParticleSystems/Gameplay/Player/P_body_bullet_impact_Big.P_body_bullet_impact_Big" (Variables|/Game/Blueprints/Pawn/Player/BP_ShooterCharacterGirl.BP_ShooterCharacterGirl_C|GetBulletHitLoc (.AsBP%20Shooter%20Character%20Girl (Utilities|Casting|CastToBP_ShooterCharacterGirl (Game|Player|GetPlayerPawn 0)))))
  (if (== (Variables|Default|GetHP) 0.0)
    (Game|SpawnActorfromClass "/Game/Blueprints/Actor/Item/BPC_Ammo.BPC_Ammo_C" (Math|Transform|MakeTransform (+ (Transformation|GetActorLocation) "0, 0,100.000000")) "AlwaysSpawn" 0 0)
    (Variables|Default|SetisDead true)
    (Pawn|Components|CharacterMovement|DisableMovement (Variables|Character|GetCharacterMovement))
    (Collision|SetCollisionEnabled (Variables|Default|GetSphereCollision) "NoCollision")
    (Physics|SetSimulatePhysics _mesh true)
    (Physics|AddImpulseatLocation _mesh (* (Transformation|GetActorForwardVector) -2e+04) (Transformation|GetWorldLocation (Variables|Character|GetMesh)) "spine_02")
    (Actor|SetLifeSpan 5.0)))

(event EventBeginPlay
  (Utilities|FlowControl|Sequence
    (:then_0
      (Utilities|Time|SetTimerbyFunctionName 0 "c_SphereColScaleUp" 0.05 true))
    (:then_1
      (bind _returnvalue (Rendering|Material|CreateDynamicMaterialInstance (Variables|Character|GetMesh) 0 0 :!class /Script/Engine.PrimitiveComponent))
      (Variables|Default|SetMI_Body _returnvalue))
    (:then_2
      (|SetRandomSpeed))
    (:then_3
      (Class|PhysicalAnimationComponent|SetSkeletalMeshComponent (Variables|Default|GetPhysicalAnimation) (Variables|Character|GetMesh)))))

(event EventAttackStart
  (CallFunction|AttackTrace))

(fn ConstructionScript)

(fn AttackTrace
  (bind _returnvalue (Transformation|GetActorLocation))
  (bind _index (Utilities|FlowControl|ForLoopwithBreak 0 (- (Variables|Default|GetNumOfAttackTraceLoop) 1) :!label _label)
    (:LoopBody
      (bind (_outhit _returnvalue_2) (Collision|LineTraceByChannel _returnvalue (+ _returnvalue (* (Math|Vector|GetForwardVector (Math|Rotator|CombineRotators (Transformation|GetActorRotation) (Math|Rotator|MakeRotator 0.0 0.0 (- (* _index (Math|Conversions|ToFloat(Integer) (/ 180 (Variables|Default|GetNumOfAttackTraceLoop)))) 9e+01)))) 1.5e+02)) "TraceTypeQuery1" false 0 "ForDuration"))
      (if _returnvalue_2
        (if (== (.HitActor (Collision|BreakHitResult _outhit)) (Game|Player|GetPlayerPawn 0))
          (Game|Damage|ApplyDamage (.HitActor (Collision|BreakHitResult _outhit)) (Math|Random|RandomFloatinRange 5.0 1e+01) 0 self)
          (goto _label Break))))))